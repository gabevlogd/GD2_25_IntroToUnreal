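; BP_DamageOverTimeTrigger is a box trigger volume that deals continuous damage to actors standing inside it.
; Box overlap events add and remove actors in a tracked list.
; Tick applies DamagePerSeconds scaled by delta time to each tracked actor, with the trigger as damage causer.
; Ticking is switched off at BeginPlay, enabled on overlap, and disabled again when the list empties.
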(event OnComponentBeginOverlap(Box)
  (params (OverlappedComponent :type Primitive%20Component%20Object%20Reference) (OtherActor :type Actor%20Object%20Reference) (OtherComp :type Primitive%20Component%20Object%20Reference) (OtherBodyIndex :type Integer) (bFromSweep :type Boolean) (SweepResult :type Hit%20Result%20Structure%20%28by%20ref%29))
  (Utilities|Array|AddUnique (Variables|Default|GetActorToHit) OtherActor)
  (Actor|Tick|SetActorTickEnabled true))

(event OnComponentEndOverlap(Box)
  (params (OverlappedComponent :type Primitive%20Component%20Object%20Reference) (OtherActor :type Actor%20Object%20Reference) (OtherComp :type Primitive%20Component%20Object%20Reference) (OtherBodyIndex :type Integer))
  (Utilities|Array|RemoveItem (Variables|Default|GetActorToHit) OtherActor)
  (if (Utilities|Array|IsEmpty (Variables|Default|GetActorToHit))
    (Actor|Tick|SetActorTickEnabled false)))

(event EventTick
  (params (DeltaSeconds :type Float%20%28single-precision%29))
  (for _array_element (Variables|Default|GetActorToHit)
    (Game|Damage|ApplyDamage _array_element (* (Variables|Default|GetDamagePerSeconds) (Utilities|Time|GetWorldDeltaSeconds)) 0 self)))

(event EventBeginPlay
  (Actor|Tick|SetActorTickEnabled false))

(fn ConstructionScript)