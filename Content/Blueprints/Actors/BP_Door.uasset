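; Interactable door actor that swings DoorPivot between closed and open yaw angles.
; Init sets the starting pose from IsOpen and configures the DoorAnimation timeline at runtime with length, float curve and bound events.
; Interact plays or reverses the timeline, or negates its play rate mid-swing; ticks lerp the yaw and completion toggles IsOpen.
; Animation start and mid-swing reversal share a RadialBurst effect spawned at the pivot.
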(event Custom|OnDoorAnimationComplete
  ;[0.1771 0.1771 0.1771] Animation Completed: Event triggered at the end of the timeline
  (Variables|Default|SetbIsOpen (not (Variables|Default|GetbIsOpen))))

(event Custom|OnDoorAnimationTick
  (params (Time :type Float%20%28single-precision%29))
  ;[0.151 0.151 0.151] Animation Tick: Event tiggered during timeline update
  (Transformation|SetRelativeRotation (Variables|Default|GetDoorPivot) (Math|Rotator|MakeRotator 0.0 0.0 (Math|Float|Lerp (Variables|Default|GetDoorCloseRelativeAngle) (Variables|Default|GetDoorOpenRelativeAngle) (/ Time (Components|Timeline|GetTimelineLength (Variables|Default|GetDoorAnimation))))) false false))

(event Custom|OnDoorAnimationStart
  ;[0.2135 0.2135 0.2135] Animation Start: Event triggered at the start of the timeline
  (if (Audio|Components|Audio|IsPlaying (Variables|Default|GetDoorAnimation))
    ;[0 0 0] Just a random example (free will)
    (Niagara|SpawnSystematLocation "/Niagara/DefaultAssets/Templates/Systems/RadialBurst.RadialBurst" (Transformation|GetWorldLocation (Variables|Default|GetDoorPivot)) "0, 0, 0" "1.000000,1.000000,1.000000" true true "AutoRelease")))

(event Custom|OnDoorAnimationReversed
  ;[0.1927 0.1927 0.1927] Animation Reversed: Event triggered when the timeline is re-triggered during playing and so reversed
  ;[0 0 0] Just a random example (free will)
  (Niagara|SpawnSystematLocation "/Niagara/DefaultAssets/Templates/Systems/RadialBurst.RadialBurst" (Transformation|GetWorldLocation (Variables|Default|GetDoorPivot)) "0, 0, 0" "1.000000,1.000000,1.000000" true true "AutoRelease"))

(event EventBeginPlay
  ;[0.2135 0.2135 0.2135] Initialization
  (CallFunction|Init))

(event EventInteract
  ;[0.1667 0.1667 0.1667] Interact Event: Play the time line for door animation based on IsOpen value
  (if (Audio|Components|Audio|IsPlaying (Variables|Default|GetDoorAnimation))
    (Components|Timeline|SetPlayRate (Variables|Default|GetDoorAnimation) (* (Components|Animation|GetPlayRate (Variables|Default|GetDoorAnimation)) -1.0))
    (CallFunction|OnDoorAnimationReversed)
    (elif (Variables|Default|GetbIsOpen)
      (Timeline|DoorAnimation Reverse)
      (else
        (Timeline|DoorAnimation Play)))))

(fn ConstructionScript)

(fn Init
  ;[0.6406 0.6406 0.6406] Set initial conditions
  (Transformation|SetRelativeRotation (Variables|Default|GetDoorPivot) (Math|Rotator|MakeRotator 0.0 0.0 (Math|Float|SelectFloat (Variables|Default|GetDoorOpenRelativeAngle) (Variables|Default|GetDoorCloseRelativeAngle) (Variables|Default|GetbIsOpen))) false false)
  (Components|Timeline|SetPlaybackPosition (Variables|Default|GetDoorAnimation) (Math|Float|SelectFloat (Variables|Default|GetDoorAnimationDuration) 0.0 (Variables|Default|GetbIsOpen)) false false)
  (Components|Timeline|SetTimelineLength (Variables|Default|GetDoorAnimation) (Variables|Default|GetDoorAnimationDuration))
  ;[0.5208 0.5208 0.5208] Binding to timeline events
  (Class|TimelineComponent|SetTimelineFinishedFunc (Variables|Default|GetDoorAnimation) (EventDispatchers|CreateEvent :!event Custom|OnDoorAnimationComplete))
  (Class|TimelineComponent|AddInterpFloat (Variables|Default|GetDoorAnimation) "/Game/Blueprints/Actors/C_TimeLineLerp.C_TimeLineLerp" (EventDispatchers|CreateEvent :!event Custom|OnDoorAnimationTick) "Time" "Time")
  (Audio|AddEvent (Variables|Default|GetDoorAnimation) 0.0 (EventDispatchers|CreateEvent :!event Custom|OnDoorAnimationStart))
  (Audio|AddEvent (Variables|Default|GetDoorAnimation) (Variables|Default|GetDoorAnimationDuration) (EventDispatchers|CreateEvent :!event Custom|OnDoorAnimationStart)))