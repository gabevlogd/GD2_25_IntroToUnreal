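; Trigger volume actor that heals actors standing inside its box over time.
; Box overlap events add and remove actors from a tracked list, toggling actor tick so it only runs while the list is non-empty.
; Each tick, every tracked actor with a BP_HealthComponent gains health at a per-second rate scaled by world delta time.
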(event OnComponentBeginOverlap(Box)
  (params (OverlappedComponent :type Primitive%20Component%20Object%20Reference) (OtherActor :type Actor%20Object%20Reference) (OtherComp :type Primitive%20Component%20Object%20Reference) (OtherBodyIndex :type Integer) (bFromSweep :type Boolean) (SweepResult :type Hit%20Result%20Structure%20%28by%20ref%29))
  (Utilities|Array|AddUnique (Variables|Default|GetActorToHeal) OtherActor)
  (Actor|Tick|SetActorTickEnabled true))

(event OnComponentEndOverlap(Box)
  (params (OverlappedComponent :type Primitive%20Component%20Object%20Reference) (OtherActor :type Actor%20Object%20Reference) (OtherComp :type Primitive%20Component%20Object%20Reference) (OtherBodyIndex :type Integer))
  (Utilities|Array|RemoveItem (Variables|Default|GetActorToHeal) OtherActor)
  (if (Utilities|Array|IsEmpty (Variables|Default|GetActorToHeal))
    (Actor|Tick|SetActorTickEnabled false)))

(event EventTick
  (params (DeltaSeconds :type Float%20%28single-precision%29))
  (for _array_element (Variables|Default|GetActorToHeal)
    (Utilities|IsValid (Actor|GetComponentbyClass _array_element "/Game/Blueprints/Components/BP_HealthComponent.BP_HealthComponent_C")
      (:Is%20Valid
        (Default|AddHealth (Actor|GetComponentbyClass _array_element "/Game/Blueprints/Components/BP_HealthComponent.BP_HealthComponent_C") (* (Variables|Default|GetHealthPerSeconds) (Utilities|Time|GetWorldDeltaSeconds)))))))

(event EventBeginPlay
  (Actor|Tick|SetActorTickEnabled false))

(fn ConstructionScript)