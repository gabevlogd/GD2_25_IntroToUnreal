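; Health component that tracks an owner's current health between a minimum and maximum, starting at maximum on BeginPlay.
; AddHealth and RemoveHealth route through SetHealth, which ignores unchanged values, stores the previous one, clamps the new one and broadcasts the change.
; Event dispatchers also announce increases, decreases and reaching either limit.
; Reaching the minimum sets IsDead, which nothing here clears.
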(event Custom|OnHealthIncreased_Event
  (Default|CallOnHealthIncreased (Variables|Default|GetCurrentHealth)))

(event Custom|OnHealthDecreased_Event
  (Default|CallOnHealthDecreased (Variables|Default|GetCurrentHealth)))

(event Custom|OnHealthReachedMax_Event
  (Default|CallOnHealthReachedMax))

(event Custom|OnHealthReachedMin_Event
  (Variables|Default|SetIsDead true)
  (Default|CallOnHealthReachedMin))

(event EventBeginPlay
  (CallFunction|Init))

(fn SetHealth
  (params (NewHelahtValue :type Float%20%28double-precision%29))
  (if (== NewHelahtValue (Variables|Default|GetCurrentHealth))
    (return)
    (else
      (LocalVariables|SetPreviousHelath (Variables|Default|GetCurrentHealth))
      (bind _output_get (Variables|Default|SetCurrentHealth (Math|Float|Clamp(Float) NewHelahtValue (Variables|Default|GetMinHealth) (Variables|Default|GetMaxHealth))))
      (Default|CallOnHealthChanged _output_get)
      (Utilities|FlowControl|Sequence
        (:then_0
          (if (== (Variables|Default|GetCurrentHealth) (Variables|Default|GetMaxHealth))
            (CallFunction|OnHealthReachedMaxEvent)
            (return)))
        (:then_1
          (if (== (Variables|Default|GetCurrentHealth) (Variables|Default|GetMinHealth))
            (CallFunction|OnHealthReachedMinEvent)
            (return)))))))

(fn AddHealth
  (params (HealthToAdd :type Float%20%28double-precision%29))
  (if (== (Variables|Default|GetCurrentHealth) (Variables|Default|GetMaxHealth))
    (return)
    (else
      (CallFunction|SetHealth (+ HealthToAdd (Variables|Default|GetCurrentHealth)))
      (CallFunction|OnHealthIncreasedEvent)
      (return))))

(fn RemoveHealth
  (params (HealthToRemove :type Float%20%28double-precision%29))
  (if (== (Variables|Default|GetCurrentHealth) (Variables|Default|GetMinHealth))
    (return)
    (else
      (CallFunction|SetHealth (- (Variables|Default|GetCurrentHealth) (Math|Float|Absolute(Float) HealthToRemove)))
      (CallFunction|OnHealthDecreasedEvent)
      (return))))

(fn Init
  (CallFunction|SetHealth (Variables|Default|GetMaxHealth)))

(fn GetCurrentHealth
  (return (Variables|Default|GetCurrentHealth)))