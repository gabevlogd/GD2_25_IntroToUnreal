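; Detector component that lets the player interact with the nearby interactable they are looking at most directly.
; TryInteract runs a multi sphere trace around the owner within the maximum interaction distance and keeps hit actors implementing BPI_Interactable.
; It scores each by the dot product of camera-to-actor direction and control rotation forward vector, then calls Interact on the highest scorer above the starting MaxDot.
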(fn TryInteract
  (bind _returnvalue (Components|GetOwner))
  (bind _returnvalue_2 (Transformation|GetActorLocation _returnvalue))
  ;[1 1 1] Detect all the interactables around the player with a multi sphere trace
  (bind _outhits (Collision|MultiSphereTraceByChannel _returnvalue_2 _returnvalue_2 (Variables|Default|GetMaxInteractionDistance) (Variables|Default|GetInteractablesTraceChannel) false (Utilities|Array|MakeArray (Components|GetOwner)) (Variables|Default|GetDraw%20Debug%20Type) true "(R=1.000000,G=0.000000,B=0.000000,A=1.000000)" "(R=0.000000,G=1.000000,B=0.000000,A=1.000000)" (Variables|Default|GetDraw%20Debug%20Time)))
  (for _array_element _outhits
    ;[1 1 1] Check if the detected actor is an interactable
    (if (Utilities|DoesObjectImplementInterface (.HitActor (Collision|BreakHitResult _array_element)) "/Game/Blueprints/Interfaces/BPI_Interactable.BPI_Interactable_C")
      ;[1 1 1] if the detected interactable is the most pointed, save the reference in the TargetActor local variable
      (if (> (Math|Vector|DotProduct (Math|Vector|Normalize (- (Transformation|GetActorLocation (.HitActor (Collision|BreakHitResult _array_element))) (Camera|GetCameraLocation (Game|GetPlayerCameraManager 0)))) (Math|Vector|GetForwardVector (Pawn|GetControlRotation (Game|GetPlayerController 0) :!class /Script/Engine.Controller))) (LocalVariables|GetMaxDot))
        (LocalVariables|SetMaxDot (Math|Vector|DotProduct (Math|Vector|Normalize (- (Transformation|GetActorLocation (.HitActor (Collision|BreakHitResult _array_element))) (Camera|GetCameraLocation (Game|GetPlayerCameraManager 0)))) (Math|Vector|GetForwardVector (Pawn|GetControlRotation (Game|GetPlayerController 0) :!class /Script/Engine.Controller))))
        (LocalVariables|SetTargetActor (.HitActor (Collision|BreakHitResult _array_element))))))
  ;[1 1 1] After the for loop if the TargetActor is a valid referece, calls the Interact method
  (Utilities|IsValid (LocalVariables|GetTargetActor)
    (:Is%20Valid
      (bind _asbpi_interactable (Utilities|Casting|CastToBPI_Interactable (LocalVariables|GetTargetActor)))
      (Default|Interact _asbpi_interactable))))