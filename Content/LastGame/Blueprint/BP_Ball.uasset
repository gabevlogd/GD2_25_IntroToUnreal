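; BP_Ball is a physics ball actor that returns to its starting spot after falling out of the map.
; On BeginPlay it records its location and binds an event to BP_GameMode's OnPlayerDeath dispatcher.
; OnFallOutOfMap teleports it to that saved location, then switches physics simulation off on its Sphere for one second before re-enabling it.
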(event Custom|OnFallOutOfMap
  (Transformation|SetActorLocation (Variables|Default|GetStartLocation) false true)
  (Physics|SetSimulatePhysics (Variables|Default|GetSphere) false)
  (Utilities|FlowControl|Delay 1.0)
  (Physics|SetSimulatePhysics (Variables|Default|GetSphere) true))

(event EventBeginPlay
  (Variables|Default|SetStartLocation (Transformation|GetActorLocation))
  (bind _asbp_game_mode (Utilities|Casting|CastToBP_GameMode (Game|GetGameMode)))
  (EventDispatchers|BindEventtoOnPlayerDeath _asbp_game_mode (EventDispatchers|CreateEvent :!event Custom|OnFallOutOfMap)))

(fn ConstructionScript)