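; BP_MovablePlane is a tiltable platform for a ball game, steered by player input.
; It binds to the player controller's move input, rotating the Plane by frame-time-scaled pitch and roll, then clamping actor rotation to a limited tilt with zero yaw.
; The game mode's player-death event resets it to level.
; A ball overlapping its Finish component only prints a game-over message.
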(event OnComponentBeginOverlap(Finish)
  (params (OverlappedComponent :type Primitive%20Component%20Object%20Reference) (OtherActor :type Actor%20Object%20Reference) (OtherComp :type Primitive%20Component%20Object%20Reference) (OtherBodyIndex :type Integer) (bFromSweep :type Boolean) (SweepResult :type Hit%20Result%20Structure%20%28by%20ref%29))
  (Utilities|Casting|CastToBP_Ball OtherActor)
  (Development|PrintString "GAME OVER" true true "(R=1.000000,G=0.000000,B=0.163040,A=1.000000)" 1e+01))

(event Custom|Move
  (params (Input%20Value :type Vector%202D%20Structure))
  (bind _returnvalue (Transformation|GetActorRotation))
  ;[1 1 1] Plane movement
  (Transformation|AddWorldRotation (Variables|Default|GetPlane) (Math|Rotator|MakeRotator (* (.y Input%20Value) (Variables|Default|GetRollSpeed) (Utilities|Time|GetWorldDeltaSeconds) -1.0) (* (.x Input%20Value) (Variables|Default|GetPitchSpeed) (Utilities|Time|GetWorldDeltaSeconds)) 0.0) true false)
  ;;[1 1 1] Limits the max/min pitch/roll
  (Transformation|SetActorRotation (Math|Rotator|MakeRotator (Math|Float|Clamp(Float) (.roll _returnvalue) -2e+01 2e+01) (Math|Float|Clamp(Float) (.pitch _returnvalue) -2e+01 2e+01) 0.0)))

(event Custom|OnPlayerDeath
  (Transformation|SetActorRotation "0, 0, 0"))

(event EventBeginPlay
  (bind _asbp_player_controller (Utilities|Casting|CastToBP_PlayerController (Game|GetPlayerController 0)))
  (EventDispatchers|BindEventtoOnMovePlaneInput _asbp_player_controller (EventDispatchers|CreateEvent :!event Custom|Move))
  (bind _asbp_game_mode (Utilities|Casting|CastToBP_GameMode (Game|GetGameMode)))
  (EventDispatchers|BindEventtoOnPlayerDeath _asbp_game_mode (EventDispatchers|CreateEvent :!event Custom|OnPlayerDeath)))

(fn ConstructionScript)